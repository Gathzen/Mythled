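; HUD Blueprint that draws a small white crosshair at the center of the screen.
; On each DrawHUD event it draws two short lines, one horizontal and one vertical, positioned from half the screen size.
; The construction script is empty, and the HUD draws nothing else.
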(event EventDrawHUD
  (params (SizeX :type Integer) (SizeY :type Integer))
  (bind _returnvalue (/ SizeX 2))
  (bind _returnvalue_2 (/ SizeY 2))
  (bind _returnvalue_3 (Math|Conversions|ToFloat(Integer) _returnvalue_2))
  (bind _returnvalue_4 (Math|Conversions|ToFloat(Integer) _returnvalue))
  (Class|HUD|DrawLine (Math|Conversions|ToFloat(Integer) (- _returnvalue 3)) _returnvalue_3 (Math|Conversions|ToFloat(Integer) (+ _returnvalue 3)) _returnvalue_3 "(R=1.000000,G=1.000000,B=1.000000,A=1.000000)" 2.0)
  (Class|HUD|DrawLine _returnvalue_4 (Math|Conversions|ToFloat(Integer) (- _returnvalue_2 3)) _returnvalue_4 (Math|Conversions|ToFloat(Integer) (+ _returnvalue_2 3)) "(R=1.000000,G=1.000000,B=1.000000,A=1.000000)" 2.0))

(fn ConstructionScript)