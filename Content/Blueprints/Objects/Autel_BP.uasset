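; Altar object with a pillar that Aaron_bp can move through the Jump/Interact input.
; Box overlap tracks whether the player is inside and enables or disables input on the altar accordingly.
; On press, ShrineOn selects whether the PillarMotion timeline plays or reverses, though each branch rewrites the same value, so the flag never toggles here.
; Timeline updates drive the pillar's relative location and set Activated to true.
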(event OnComponentBeginOverlap(Box)
  (params (OverlappedComponent :type Primitive%20Component%20Object%20Reference) (OtherActor :type Actor%20Object%20Reference) (OtherComp :type Primitive%20Component%20Object%20Reference) (OtherBodyIndex :type Integer) (bFromSweep :type Boolean) (SweepResult :type Hit%20Result%20Structure%20%28by%20ref%29))
  (Utilities|Casting|CastToAaron_bp OtherActor)
  (Variables|Default|SetPlayerIn true)
  (Input|EnableInput (Game|GetPlayerController 0)))

(event OnComponentEndOverlap(Box)
  (params (OverlappedComponent :type Primitive%20Component%20Object%20Reference) (OtherActor :type Actor%20Object%20Reference) (OtherComp :type Primitive%20Component%20Object%20Reference) (OtherBodyIndex :type Integer))
  (Utilities|Casting|CastToAaron_bp OtherActor)
  (Variables|Default|SetPlayerIn false)
  (Input|DisableInput (Game|GetPlayerController 0)))

(event Input|ActionEvents|InputActionJump/Interact
  (params (Key :type Key%20Structure :default "None"))
  (:Pressed
    (if (Variables|Default|GetPlayerIn)
      (if (Variables|Default|GetShrineOn)
        (Variables|Default|SetShrineOn true)
        (bind _moveup (Timeline|Pillar%20motion Play)
          (:Update
            (Transformation|SetRelativeLocation (Variables|Default|GetPillar) _moveup false false)
            (Variables|Default|SetActivated true)))
        (else
          (Variables|Default|SetShrineOn false)
          (Timeline|Pillar%20motion Reverse))))))

(fn ConstructionScript)