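; Base projectile actor that homes in on the player character, Aaron, and damages it on contact.
; BeginPlay sets the player's AaronV1 component as the projectile movement's homing target.
; Sphere overlap with Aaron calls Died with Damage and destroys the projectile; overlapping the Guardian only prints a debug string, while any other actor destroys it.
; Blocking hits on the mesh or sphere also destroy it.
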(event OnComponentBeginOverlap(Sphere)
  (params (OverlappedComponent :type Primitive%20Component%20Object%20Reference) (OtherActor :type Actor%20Object%20Reference) (OtherComp :type Primitive%20Component%20Object%20Reference) (OtherBodyIndex :type Integer) (bFromSweep :type Boolean) (SweepResult :type Hit%20Result%20Structure%20%28by%20ref%29))
  (bind _asaaron_bp (Utilities|Casting|CastToAaron_bp OtherActor)
    (:then
      (Default|Died _asaaron_bp (Variables|Default|GetDamage))
      (Actor|DestroyActor))
    (:CastFailed
      (if (== OtherActor (Variables|Default|GetGuardian))
        (Development|PrintString "Hello")
        (else
          (Actor|DestroyActor))))))

(event OnComponentHit(Mesh_Projectile)
  (params (HitComponent :type Primitive%20Component%20Object%20Reference) (OtherActor :type Actor%20Object%20Reference) (OtherComp :type Primitive%20Component%20Object%20Reference) (NormalImpulse :type Vector :default "0, 0, 0") (Hit :type Hit%20Result%20Structure%20%28by%20ref%29))
  (Actor|DestroyActor))

(event OnComponentHit(Sphere)
  (params (HitComponent :type Primitive%20Component%20Object%20Reference) (OtherActor :type Actor%20Object%20Reference) (OtherComp :type Primitive%20Component%20Object%20Reference) (NormalImpulse :type Vector :default "0, 0, 0") (Hit :type Hit%20Result%20Structure%20%28by%20ref%29))
  (Actor|DestroyActor))

(event EventBeginPlay
  (Variables|/Script/Engine.ProjectileMovementComponent|SetHomingTargetComponent (Variables|Default|GetProjectileMovement) (Variables|/Game/Blueprints/Aaron_bp.Aaron_bp_C|GetAaron_V1 (.AsAaron%20Bp (Utilities|Casting|CastToAaron_bp (Game|GetPlayerCharacter 0))))))

(fn ConstructionScript)