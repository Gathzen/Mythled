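; Guardian enemy that hovers in place, turns to face the player pawn and fires projectiles at it.
; A Hover timeline started on BeginPlay offsets the actor's height.
; Tick smoothly yaws the mesh and aims FirePoint in pitch and yaw using interpolated look-at rotations.
; Tick also calls Attack, whose Delay throttles GuardianProjectile_BP spawns at the Barrel socket to the FireRate interval.
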(event Custom|UpdateRotationAttack
  (bind _returnvalue (Game|Player|GetPlayerPawn 0))
  (bind _firepoint (Variables|Default|GetFirePoint))
  (bind _returnvalue_2 (Transformation|GetWorldLocation _firepoint))
  (bind _returnvalue_3 (Transformation|GetActorLocation _returnvalue))
  (bind _returnvalue_4 (Math|Rotator|FindLookatRotation _returnvalue_2 _returnvalue_3))
  ;[1 1 1] Attack rotation
  (Transformation|SetWorldRotation _firepoint (Math|Interpolation|RInterpTo (Transformation|GetWorldRotation _firepoint) (Math|Rotator|MakeRotator 0.0 (.pitch _returnvalue_4) (.yaw _returnvalue_4)) (Variables|Default|GetDeltaTime) (Variables|TurretSettings|GetRotationSpeed)) false false))

(event Custom|Attack
  ;[1 1 1] Attack
  (Utilities|FlowControl|Delay (Variables|TurretSettings|GetFireRate))
  (Game|SpawnActorfromClass "/Game/Blueprints/Objects/GuardianProjectile_BP.GuardianProjectile_BP_C" (Transformation|GetSocketTransform (Variables|Default|GetFirePoint) "Barrel" "RTS_World") "Undefined" 0 0))

(event Custom|UpdateRotationGuardian
  (bind _guardianmesh (Variables|Default|GetGuardianMesh))
  ;[1 1 1] Guardian rotation
  (Transformation|SetWorldRotation _guardianmesh (Math|Interpolation|RInterpTo (Transformation|GetWorldRotation _guardianmesh) (Math|Rotator|MakeRotator 0.0 0.0 (.yaw (Math|Rotator|FindLookatRotation (Transformation|GetWorldLocation _guardianmesh) (Transformation|GetActorLocation (Game|Player|GetPlayerPawn 0))))) (Variables|Default|GetDeltaTime) (Variables|TurretSettings|GetRotationSpeed)) false false))

(event EventTick
  (params (DeltaSeconds :type Float%20%28single-precision%29))
  ;[1 1 1] Game Loop
  (Variables|Default|SetDeltaTime DeltaSeconds)
  (CallFunction|UpdateRotationGuardian)
  (CallFunction|UpdateRotationAttack)
  (CallFunction|Attack))

(event EventBeginPlay
  (bind _returnvalue (Transformation|GetActorLocation))
  ;[1 1 1] Hover
  (bind _float (Timeline|Hover PlayFromStart)
    (:Update
      (Transformation|SetActorLocation (Math|Vector|MakeVector (.x _returnvalue) (.y _returnvalue) (+ (.z _returnvalue) _float)) false false))))

(fn ConstructionScript)