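; Protection Blueprint is an actor with a limited Life pool that is worn down by contact with MasterP actors.
; Each Box begin overlap that casts successfully to MasterP calls Hit, which subtracts one point of Life.
; When Life is no longer above zero, Hit calls Death, which destroys the actor.
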(event OnComponentBeginOverlap(Box)
  (params (OverlappedComponent :type Primitive%20Component%20Object%20Reference) (OtherActor :type Actor%20Object%20Reference) (OtherComp :type Primitive%20Component%20Object%20Reference) (OtherBodyIndex :type Integer) (bFromSweep :type Boolean) (SweepResult :type Hit%20Result%20Structure%20%28by%20ref%29))
  (Utilities|Casting|CastToMasterP OtherActor)
  (CallFunction|Hit))

(fn ConstructionScript)

(fn Hit
  (Variables|Default|SetLife (- (Variables|Default|GetLife) 1.0))
  (if (not (> (Variables|Default|GetLife) 0.0))
    (CallFunction|Death)))

(fn Death
  (Actor|DestroyActor))